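; BP_LevelMusic is a level music actor that plays a sound wave and broadcasts OnTheDrop when its loudness exceeds a threshold.
; At BeginPlay it starts playback and precomputes amplitude buckets across the whole track.
; A looping timer, spaced at duration divided by bucket count, steps through that data in time with playback rather than analysing audio live.
; The timer is cleared when the audio finishes.
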(event Custom|OnAudioFinished_Event_0
  (Utilities|Time|ClearTimerbyFunctionName 0 "CheckSoundAmp"))

(event EventBeginPlay
  (EventDispatchers|AssignOnAudioFinished (Variables|Default|GetAudio) (delegate Custom|OnAudioFinished_Event_0))
  (CallFunction|StartCheck))

(event Collision|EventActorBeginOverlap
  (params (OtherActor :type Actor%20Object%20Reference)))

(event EventTick
  (params (DeltaSeconds :type Float%20%28single-precision%29)))

(fn ConstructionScript)

(fn ProcessSound
  (bind _wave (Variables|Default|GetWave))
  (bind _outamplitudes (Class|SoundVisualizationStatics|GetAmplitude _wave 0 0.0 (Variables|/Script/Engine.SoundBase|GetDuration _wave) (Variables|Default|GetChunks)))
  (Variables|Default|SetData _outamplitudes))

(fn CheckSoundAmp
  (if (> (Utilities|Array|Get(acopy) (Variables|Default|GetData) (Variables|Default|GetCurrentIndex)) (Variables|Default|GetThreshold))
    (Default|CallOntheDrop (Utilities|Array|Get(acopy) (Variables|Default|GetData) (Variables|Default|GetCurrentIndex))))
  (bind _result (Math|Integer|IncrementInt (Variables|Default|GetCurrentIndex))
    (:%20%20
      (if (> _result (Variables|Default|GetChunks))
        (Variables|Default|SetCurrentIndex 0)))))

(fn StartCheck
  (bind _audio (Variables|Default|GetAudio))
  (Audio|Components|Audio|SetSound _audio (Variables|Default|GetWave))
  (Audio|Components|Audio|Play _audio 0.0)
  (bind _output_get (Variables|Default|SetIntervalCheck (/ (Variables|/Script/Engine.SoundBase|GetDuration (Variables|Default|GetWave)) (Math|Conversions|ToFloat(Integer) (Variables|Default|GetChunks)))))
  (CallFunction|ProcessSound)
  (Utilities|Time|SetTimerbyFunctionName self "CheckSoundAmp" _output_get true))