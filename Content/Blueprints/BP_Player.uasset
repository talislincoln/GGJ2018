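; Player actor for a lane-switching runner that rides the spline of a BP_LevelManagerV2 track.
; Each Tick snaps it to the nearest spline point, offsets it forward by Velocity and sideways by one of three lanes, and matches spline rotation.
; UpdateVelocity doubles the capped score multiplier on boosts or resets it otherwise, eases camera FOV by timeline, and recovers lost speed by timer.
; Score accumulates every frame and updates the HUD.
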(event Custom|UpdateFOV
  (bind _velocity (Variables|Default|GetVelocity))
  (bind _defaultspeed (Variables|Default|GetDefaultSpeed))
  (bind _fovfactor (Variables|Default|GetFOVFactor))
  (bind _defaultfov (Variables|Default|GetDefaultFOV))
  (bind _returnvalue (/ _velocity _defaultspeed))
  (bind _returnvalue_2 (* _returnvalue _fovfactor))
  ;[1 1 1] Update FOV
  (bind _alpha (Timeline|FOV_Timeline Play)
    (:Update
      (if (< _returnvalue 1.0) ; If speed is to low
        (Camera|SetFieldOfView (Variables|Default|GetCamera) (Math|Float|Lerp (Variables|Default|GetCurrentFOV) (Math|Float|Clamp(Float) (+ _defaultfov _returnvalue_2) 6e+01 1e+02) _alpha))
        (Variables|Default|SetCurrentFOV (Math|Float|Lerp (Variables|Default|GetCurrentFOV) (Math|Float|Clamp(Float) (+ _defaultfov _returnvalue_2) 6e+01 1e+02) _alpha))
        (else
          (Camera|SetFieldOfView (Variables|Default|GetCamera) (Math|Float|Lerp (Variables|Default|GetCurrentFOV) (Math|Float|Clamp(Float) (- _defaultfov _returnvalue_2) 6e+01 1e+02) _alpha))
          (Variables|Default|SetCurrentFOV (Math|Float|Lerp (Variables|Default|GetCurrentFOV) (Math|Float|Clamp(Float) (- _defaultfov _returnvalue_2) 6e+01 1e+02) _alpha)))))))

(event EventBeginPlay
  ;[1 1 1] Begin Play
  (bind _returnvalue (UserInterface|CreateWidget "/Game/UI/Widgets/BP_MainHUD.BP_MainHUD_C" (Game|GetPlayerController 0)))
  (UserInterface|Viewport|AddtoViewport _returnvalue 0)
  (Variables|Default|SetPlayerHUD _returnvalue)
  (Variables|Default|SetVelocity (Variables|Default|GetDefaultSpeed))
  (bind _outactors (Actor|GetAllActorsOfClass "/Game/Blueprints/Level/BP_LevelManagerV2.BP_LevelManagerV2_C"))
  (if (> (Utilities|Array|Length _outactors) 0)
    (bind _output_get (Variables|Default|SetTrackRef (Utilities|Array|Get(acopy) _outactors)))
    (Transformation|SetActorLocation (Transformation|GetActorLocation _output_get) false false)
    (bind _output_get_2 (Variables|Default|SetCurrentFOV (Variables|/Script/Engine.CameraComponent|GetFieldOfView (Variables|Default|GetCamera))))
    (Variables|Default|SetDefaultFOV _output_get_2)))

(event EventTick
  (params (DeltaSeconds :type Float%20%28single-precision%29))
  ;[1 1 1] Ray tracing and updating player position on Tick
  (CallFunction|IncreaseScore)
  (Utilities|IsValid (Variables|Default|GetTrackRef)
    (:Is%20Valid
      (Transformation|SetActorLocation (CallFunction|GetSplineLocation) false false)
      (Transformation|AddActorWorldOffset (CallFunction|GetNextSplineDirection))
      (Transformation|SetActorRotation (CallFunction|GetNextSplineRotation)))))

(event Input|ActionEvents|InputActionLeft
  (params (Key :type Key%20Structure))
  ;[1 1 1] Handle player input
  (:Pressed
    (Variables|Default|SetCurrentPosition (Math|Integer|Max(Integer) (- (Variables|Default|GetCurrentPosition) 1) -1))))

(event Input|ActionEvents|InputActionRight
  (params (Key :type Key%20Structure))
  ;[1 1 1] Handle player input
  (:Pressed
    (Variables|Default|SetCurrentPosition (Math|Integer|Min(Integer) (+ (Variables|Default|GetCurrentPosition) 1) 1))))

(event Input|KeyboardEvents|Q
  (params (Key :type Key%20Structure))
  (:Pressed
    (bind _asbp_game_mode (Utilities|Casting|CastToBP_GameMode (Game|GetGameMode)))
    (Default|AddScore _asbp_game_mode self)))

(event Input|KeyboardEvents|F
  (params (Key :type Key%20Structure))
  (:Pressed
    (Variables|Default|SetVelocity (+ (Variables|Default|GetVelocity) 5.0))))

(fn ConstructionScript)

(fn UpdateVelocity
  (params (VelocityPercentage :type Float%20%28single-precision%29))
  (if (> VelocityPercentage 1.0)
    (Variables|Default|SetScoreMultiplier (Math|Float|Clamp(Float) (* (Variables|Default|GetScoreMultiplier) 2.0) 1.0 32.0))
    (else
      (Variables|Default|SetScoreMultiplier 1.0)))
  (Variables|Default|SetVelocity (Math|Float|Clamp(Float) (* VelocityPercentage (Variables|Default|GetVelocity)) 0.0 (Variables|Default|GetMaxSpeed)))
  (CallFunction|BackupVelocity))

(fn BackupVelocity
  (CallFunction|UpdateFOV)
  (if (< (Variables|Default|GetVelocity) (Variables|Default|GetDefaultSpeed))
    (Variables|Default|SetVelocity (Math|Float|Min(Float) (+ (Variables|Default|GetVelocity) (Variables|Default|GetIncrementAmount)) (Variables|Default|GetDefaultSpeed)))
    (Utilities|Time|SetTimerbyFunctionName self "BackupVelocity" (Variables|Default|GetIncrementRate))))

(fn GetNextSplineDirection
  (return (+ (* (Spline|FindDirectionClosesttoWorldLocation (Variables|/Game/Blueprints/Level/BP_LevelManagerV2.BP_LevelManagerV2_C|GetSpline (Variables|Default|GetTrackRef)) (Transformation|GetActorLocation) "World") (Variables|Default|GetVelocity)) (* (Transformation|GetActorUpVector) 25.0) (* (* (Transformation|GetActorRightVector) (Variables|Default|GetCurrentPosition)) (* (Math|Float|MakeLiteralFloat 1.5e+02) (.x (Transformation|GetActorScale3D (Variables|Default|GetTrackRef))))) (* (Transformation|GetActorUpVector) (* (Math|Integer|Absolute(Integer) (Variables|Default|GetCurrentPosition)) 50)))))

(fn GetNextSplineRotation
  (return (Class|SplineComponent|FindRotationClosesttoWorldLocation (Variables|/Game/Blueprints/Level/BP_LevelManagerV2.BP_LevelManagerV2_C|GetSpline (Variables|Default|GetTrackRef)) (Transformation|GetActorLocation) "World")))

(fn GetSplineLocation
  (return (Spline|FindLocationClosesttoWorldLocation (Variables|/Game/Blueprints/Level/BP_LevelManagerV2.BP_LevelManagerV2_C|GetSpline (Variables|Default|GetTrackRef)) (Transformation|GetActorLocation) "World")))

(fn CheckFloor)

(fn IncreaseScore
  (bind _playerhud (Variables|Default|GetPlayerHUD))
  (bind _output_get (Variables|Default|SetScore (+ (Variables|Default|GetScoreMultiplier) (Variables|Default|GetScore))))
  (Rendering|Components|TextRender|SetText (Variables|/Game/UI/Widgets/BP_MainHUD.BP_MainHUD_C|GetCurrentScoreText _playerhud) (Utilities|Text|ToText(Float) _output_get "HalfToEven"))
  (Rendering|Components|TextRender|SetText (Variables|/Game/UI/Widgets/BP_MainHUD.BP_MainHUD_C|GetMultiplierText _playerhud) (Utilities|Text|FormatText "{0} X" (Variables|Default|GetScoreMultiplier))))