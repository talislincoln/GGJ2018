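; BP_PhotoParticles is a music-reactive particle actor driven by the level music's drop event.
; On BeginPlay it seeds a random stream from real time and binds to OnTheDrop on the first BP_LevelMusic found.
; Each drop scales the incoming value down to set Color, Scale and Acceleration parameters, randomizing color channels and acceleration axes through the stream.
; The handler also prints debug values on screen.
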(event Custom|OnTheDrop_Event_0
  (params (Value :type Float%20%28single-precision%29))
  (bind _returnvalue (* Value 0.0001))
  (bind _speed (Variables|Default|GetSpeed))
  (bind _randstream (Variables|Default|GetRandStream))
  (bind _randstream_2 (Variables|Default|GetRandStream))
  (bind _particlesystem (Variables|Default|GetParticleSystem))
  (bind _returnvalue_2 (Math|Random|RandomFloatinRangefromStream -1.0 1.0 _randstream_2))
  (bind _returnvalue_3 (Math|Random|RandomFloatinRangefromStream 0.25 2.0 _randstream))
  (bind _returnvalue_4 (* _returnvalue _speed))
  (bind _returnvalue_5 (* _returnvalue_4 _returnvalue_2))
  (bind _returnvalue_6 (* _returnvalue _returnvalue_3))
  (Effects|Components|ParticleSystem|SetColorParameter _particlesystem "Color" (Utilities|Struct|MakeLinearColor _returnvalue_6 _returnvalue_6 _returnvalue_6 1.0))
  (Development|PrintString (Utilities|String|ToString(Float) _returnvalue))
  (Development|PrintString (Utilities|String|ToString(Float) _returnvalue_6) true true "(R=0.842601,G=1.000000,B=0.000000,A=1.000000)")
  (Effects|Components|ParticleSystem|SetVectorParameter _particlesystem "Scale" (Math|Conversions|ToVector(Float) (* _returnvalue (Variables|Default|GetScaling))))
  (Effects|Components|ParticleSystem|SetVectorParameter (Variables|Default|GetParticleSystem) "Acceleration" (Math|Vector|MakeVector _returnvalue_5 _returnvalue_5 _returnvalue_5)))

(event EventBeginPlay
  (bind _returnvalue (Utilities|Time|GetRealTimeSeconds))
  (bind _returnvalue_2 (Math|Float|Truncate _returnvalue))
  (bind _output_get (Variables|Default|SetRandStream (Math|Random|MakeRandomStream _returnvalue_2)))
  (Math|Random|SetRandomStreamSeed _output_get _returnvalue_2)
  (bind _outactors (Actor|GetAllActorsOfClass "/Game/Audio/BP_LevelMusic.BP_LevelMusic_C"))
  (if (> (Utilities|Array|Length _outactors) 0)
    (EventDispatchers|AssignOntheDrop (Utilities|Array|Get(acopy) _outactors) (delegate Custom|OnTheDrop_Event_0))))

(event Collision|EventActorBeginOverlap
  (params (OtherActor :type Actor%20Object%20Reference)))

(event EventTick
  (params (DeltaSeconds :type Float%20%28single-precision%29)))

(fn ConstructionScript)