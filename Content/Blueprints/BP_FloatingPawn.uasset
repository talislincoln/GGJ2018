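; BP_FloatingPawn is an actor that wanders on its own, drifting constantly forward while periodically turning to random orientations.
; A looping timer started on BeginPlay picks a random rotation, including roll, and the Rotation timeline blends the actor from its current rotation to that target.
; Tick offsets the actor along its forward vector by Speed each frame, without delta-time scaling or collision sweep.
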(event Custom|NewRotation
  (bind _output_get (Variables|Default|SetDesiredRotation (Math|Random|RandomRotator true)))
  (bind _output_get_2 (Variables|Default|SetCurrentRotation (Transformation|GetActorRotation)))
  (bind _newtrack_0 (Timeline|Rotation PlayFromStart)
    (:Update
      (Transformation|SetActorRotation (Math|Rotator|Lerp(Rotator) _output_get_2 _output_get _newtrack_0)))))

(event EventBeginPlay
  (Utilities|Time|SetTimerbyEvent (delegate Custom|NewRotation) 4.9 true))

(event EventTick
  (params (DeltaSeconds :type Float%20%28single-precision%29))
  (Transformation|AddActorWorldOffset (* (Transformation|GetActorForwardVector) (Variables|Default|GetSpeed))))

(fn ConstructionScript)