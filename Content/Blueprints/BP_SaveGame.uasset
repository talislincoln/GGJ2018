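; BP_SaveGame is a save game Blueprint that holds a HighScores list and adds new score entries to it.
; AddScore scans the list and, at the first entry the new score beats, appends it to the end rather than inserting it there, then breaks.
; A follow-up index check also appends when the list has fewer than ten entries; the function never sorts or trims the list.
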(fn AddScore
  (params (NewScore :type Score%20Data%20Structure))
  (bind _highscores (Variables|Default|GetHighScores))
  (bind _returnvalue (Utilities|Array|Length _highscores))
  (bind _index (Utilities|FlowControl|ForLoopwithBreak 0 (- _returnvalue 1) :!label _label)
    (:LoopBody
      (if (> (.Score (Utilities|Struct|BreakScoreData NewScore)) (.score (Utilities|Array|Get(acopy) _highscores _index)))
        (Utilities|Array|Add _highscores NewScore)
        (goto _label Break)))
    (:Completed
      (if (>= _index _returnvalue)
        (if (< _returnvalue 10)
          (Utilities|Array|Add _highscores NewScore))))))