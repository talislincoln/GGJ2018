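; Base obstacle actor that hits players with a configurable debuff when they run into it in its lane.
; On collider overlap, it checks that the player's current position matches its lane, then passes the debuff and player to BP_GameMode through CallOnPowerHit.
; ApplyBuff and RemoveBuff scale player velocity by the debuff's modifier and its inverse, but their only callers, in a hide-delay-destroy chain, are disconnected and never run.
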(event OnComponentBeginOverlap(Collider)
  (params (OverlappedComponent :type Primitive%20Component%20Object%20Reference) (OtherActor :type Actor%20Object%20Reference) (OtherComp :type Primitive%20Component%20Object%20Reference) (OtherBodyIndex :type Integer) (bFromSweep :type Boolean) (SweepResult :type Hit%20Result%20Structure%20%28by%20ref%29))
  (bind _asbp_game_mode (Utilities|Casting|CastToBP_GameMode (Game|GetGameMode)))
  (bind _asbp_player (Utilities|Casting|CastToBP_Player OtherActor))
  (if (not (!= (Variables|/Game/Blueprints/BP_Player.BP_Player_C|GetCurrentPosition _asbp_player) (Variables|Default|GetLane)))
    (Default|CallOnPowerHit _asbp_game_mode (Variables|Power|GetPowerDebuff) _asbp_player)))

(fn ConstructionScript)

(fn ApplyBuff
  (params (PlayerRef :type Actor%20Object%20Reference))
  (bind _asbp_player (Utilities|Casting|CastToBP_Player PlayerRef))
  (Variables|/Game/Blueprints/BP_Player.BP_Player_C|SetVelocity _asbp_player (* (Variables|/Game/Blueprints/BP_Player.BP_Player_C|GetVelocity _asbp_player) (.velocitymodifier (Variables|Power|GetPowerDebuff)))))

(fn RemoveBuff
  (params (PlayerRef :type Actor%20Object%20Reference))
  (bind _asbp_player (Utilities|Casting|CastToBP_Player PlayerRef))
  (Variables|/Game/Blueprints/BP_Player.BP_Player_C|SetVelocity _asbp_player (* (Variables|/Game/Blueprints/BP_Player.BP_Player_C|GetVelocity _asbp_player) (/ 1.0 (.velocitymodifier (Variables|Power|GetPowerDebuff))))))