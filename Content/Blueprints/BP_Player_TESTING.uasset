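; Test player Blueprint that moves by axis input and has a Left Shift speed boost.
; Vertical and Horizontal axes share one SetActorLocation that offsets X and Y by axis value times Velocity per call, without delta-time scaling.
; Pressing Shift doubles Velocity, plays a world camera shake and narrows camera FOV through the FOV_Zoom timeline.
; Releasing Shift restores Velocity and reverses the zoom.
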(event Input|AxisEvents|InputAxisHorizontal
  (params (AxisValue :type Float%20%28single-precision%29))
  (bind _returnvalue (Transformation|GetActorLocation))
  (Transformation|SetActorLocation (Math|Vector|MakeVector (+ (* (stale Input|AxisEvents|InputAxisVertical AxisValue) (Variables|Default|GetVelocity)) (.x _returnvalue)) (+ (.y _returnvalue) (* AxisValue (Variables|Default|GetVelocity))) (.z _returnvalue)) false false))

(event Input|AxisEvents|InputAxisVertical
  (params (AxisValue :type Float%20%28single-precision%29))
  (bind _returnvalue (Transformation|GetActorLocation))
  (Transformation|SetActorLocation (Math|Vector|MakeVector (+ (* AxisValue (Variables|Default|GetVelocity)) (.x _returnvalue)) (+ (.y _returnvalue) (* (stale Input|AxisEvents|InputAxisHorizontal AxisValue) (Variables|Default|GetVelocity))) (.z _returnvalue)) false false))

(event Input|KeyboardEvents|LeftShift
  (params (Key :type Key%20Structure))
  (:Pressed
    (Variables|Default|SetVelocity 1e+01)
    (Camera|PlayWorldCameraShake "/Game/Blueprints/BP_PlayerSpeedUpCameraShake.BP_PlayerSpeedUpCameraShake_C" "0, 0, 0" 0.0 5e+03)
    (bind _alpha (Timeline|FOV_Zoom Play)
      (:Update
        (Camera|SetFieldOfView (Variables|Default|GetCamera) (Math|Float|Lerp 9e+01 6e+01 _alpha)))))
  (:Released
    (Variables|Default|SetVelocity 5.0)
    (Timeline|FOV_Zoom Reverse)))

(fn ConstructionScript)