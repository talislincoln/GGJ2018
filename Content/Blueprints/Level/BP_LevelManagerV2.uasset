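; Level manager that procedurally builds a winding spline road meant to keep extending as the player moves.
; BeginPlay lays points in random cone directions, adding a random road spline mesh and a BP_PhotoParticles actor along them.
; A one-second timer runs RunMapGeneration to trim points behind the player, append new ones and reposition existing meshes and particles as a recycled pool.
; Spline save/load helpers and an L-key hook support testing.
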(event EventBeginPlay
  (bind _outactors (Actor|GetAllActorsOfClass "/Game/Blueprints/BP_Player.BP_Player_C"))
  (Variables|Default|SetPlayerRef (Utilities|Array|Get(acopy) _outactors))
  (CallFunction|GenerateLevelSpline 2e+03 50 "1.000000, 0, 0")
  (CallFunction|GenerateLevelSplineMesh)
  (Utilities|Time|SetTimerbyFunctionName self "RunMapGeneration" 1.0 true))

(event Collision|EventActorBeginOverlap
  (params (OtherActor :type Actor%20Object%20Reference)))

(event EventTick
  (params (DeltaSeconds :type Float%20%28single-precision%29)))

(event Input|KeyboardEvents|B
  (params (Key :type Key%20Structure)))

(event Input|KeyboardEvents|L
  (params (Key :type Key%20Structure))
  (:Pressed
    (Class|SplineComponent|AddPoints (Variables|Default|GetSpline) (Variables|Default|GetTestPoints) true)
    (CallFunction|GenerateLevelSplineMesh)))

(fn ConstructionScript)

(fn GenerateLevelSpline
  (params (RoadLength :type Float%20%28single-precision%29) (NumOfRoad :type Integer) (GeneralDirection :type Vector))
  (bind _spline (Variables|Default|GetSpline))
  (Utilities|FlowControl|ForLoopwithBreak 0 NumOfRoad
    (:LoopBody
      (Spline|AddSplinePoint (Variables|Default|GetSpline) (+ (Spline|GetLocationatSplinePoint _spline (- (Spline|GetNumberOfSplinePoints _spline) 1) "Local") (* (Math|Random|RandomUnitVectorinConeinDegrees GeneralDirection (Math|Random|RandomFloatinRange 0.0 1e+01)) RoadLength)) "Local" true))))

(fn GenerateLevelSplineMesh
  (bind _roadmeshes (Variables|Default|GetRoadMeshes))
  (bind _returnvalue (Utilities|Array|Length _roadmeshes))
  (bind _returnvalue_2 (- _returnvalue 1))
  (bind _returnvalue_3 (Math|Random|RandomIntegerinRange 0 _returnvalue_2))
  (bind _output (Utilities|Array|Get(acopy) _roadmeshes _returnvalue_3))
  (for _index (range 1 (- (Spline|GetNumberOfSplinePoints (Variables|Default|GetSpline)) 2))
    (bind _returnvalue_4 (AddComponent|AddSplineMeshComponent false))
    (Components|StaticMesh|SetStaticMesh _returnvalue_4 _output)
    (for _index_2 (range 0 (Rendering|Material|GetNumMaterials _returnvalue_4))
      (Rendering|Material|SetMaterial _returnvalue_4 _index_2 (Rendering|Material|GetMaterial _output _index_2)))
    (Utilities|Array|Add (Variables|Default|GetSplineMeshes) _returnvalue_4)
    (bind _returnvalue_5 (Game|SpawnActorfromClass "/Game/Blueprints/Particles/BP_PhotoParticles.BP_PhotoParticles_C" (Math|Transform|MakeTransform (Spline|GetLocationatSplinePoint (Variables|Default|GetSpline) _index "World") "0, 0, 0" "1,1,1") "AlwaysSpawn" 0 0))
    (Utilities|Array|Add (Variables|Default|GetPhotoParticles) _returnvalue_5))
  (CallFunction|RearrangeCurrentMeshes))

(fn LoadSplines
  (params (NewParam :type Array%20of%20Spline%20Point%20Structures))
  (bind _spline (Variables|Default|GetSpline))
  (Spline|ClearSplinePoints _spline true)
  (Class|SplineComponent|AddPoints _spline NewParam true))

(fn ClearandSaveSplines
  (bind _splinemeshes (Variables|Default|GetSplineMeshes))
  (bind _spline (Variables|Default|GetSpline))
  (Utilities|Array|Clear (Variables|Default|GetTestPoints))
  (for _index (range 0 (- (Spline|GetNumberOfSplinePoints (Variables|Default|GetSpline)) 1))
    (Utilities|Array|Add (Variables|Default|GetTestPoints) (Utilities|Struct|MakeSplinePoint (Class|SplineComponent|FindInputKeyClosesttoWorldLocation _spline (Spline|GetLocationatSplinePoint _spline _index "Local")) (Spline|GetLocationatSplinePoint _spline _index "Local") (Spline|GetArriveTangentatSplinePoint _spline _index "Local") (Spline|GetLeaveTangentatSplinePoint _spline _index "Local") (Spline|GetRotationatSplinePoint _spline _index "Local") (Spline|GetScaleatSplinePoint _spline _index) (Class|SplineComponent|GetSplinePointType _spline _index))))
  (Spline|ClearSplinePoints (Variables|Default|GetSpline) true)
  (for _array_element _splinemeshes
    (Components|DestroyComponent _array_element))
  (Utilities|Array|Clear _splinemeshes))

(fn PlayerCheckAgainstSpline
  (params (DistanceCheck :type Float%20%28single-precision%29) (SplinePointIndex :type Integer))
  (bind _spline (Variables|Default|GetSpline))
  (return (< (Math|Vector|VectorLength (- (Transformation|GetActorLocation (Variables|Default|GetPlayerRef)) (Spline|GetLocationatDistanceAlongSpline _spline (Spline|GetDistanceAlongSplineatSplinePoint _spline SplinePointIndex) "Local"))) DistanceCheck)))

(fn LevelCheck
  (CallFunction|RemoveSplinesfromStart 10)
  (CallFunction|GenerateLevelSpline 1e+02 10 (Math|Random|RandomUnitVector))
  (CallFunction|GenerateLevelSplineMesh))

(fn RemoveSplinesfromStart
  (params (NumOfSplines :type Integer))
  (bind _splinemeshes (Variables|Default|GetSplineMeshes))
  (bind _index (Utilities|FlowControl|ForLoopwithBreak 0 (- (Math|Float|Truncate (Class|SplineComponent|FindInputKeyClosesttoWorldLocation (Variables|Default|GetSpline) (Transformation|GetActorLocation (Variables|Default|GetPlayerRef)))) 2))
    (:LoopBody
      (Math|Integer|IncrementInt (LocalVariables|GetAmountRemoved)
        (:%20%20
          (Spline|RemoveSplinePoint (Variables|Default|GetSpline) _index true))))
    (:Completed
      (for _index_2 (range 0 (- (LocalVariables|GetAmountRemoved) 1))
        (bind _output_get (LocalVariables|SetTemp (Utilities|Array|Get(acopy) _splinemeshes)))
        (Utilities|Array|RemoveIndex _splinemeshes)
        (Utilities|Array|Add _splinemeshes _output_get)))))

(fn GenerateLevelSplineMeshSet
  (params (StartIndex :type Integer) (Num :type Integer))
  (bind _returnvalue (+ StartIndex Num))
  (bind _splinemeshes (Variables|Default|GetSplineMeshes))
  (bind _spline (Variables|Default|GetSpline))
  (bind _spline_2 (Variables|Default|GetSpline))
  (bind _roadmeshes (Variables|Default|GetRoadMeshes))
  (bind _returnvalue_2 (Spline|GetNumberOfSplinePoints _spline))
  (for _index (range StartIndex (- (Math|Integer|SelectInt _returnvalue (- _returnvalue_2 1) (> _returnvalue _returnvalue_2)) 1))
    (bind _returnvalue_3 (AddComponent|AddSplineMeshComponent false))
    (Components|StaticMesh|SetStaticMesh _returnvalue_3 (Utilities|Array|Get(acopy) _roadmeshes (Math|Random|RandomIntegerinRange 0 (- (Utilities|Array|Length _roadmeshes) 1))))
    (bind _returnvalue_4 (Utilities|Array|Add _splinemeshes _returnvalue_3))
    (SplineMesh|SetStartandEnd (Utilities|Array|Get(acopy) _splinemeshes _returnvalue_4) (Spline|GetLocationatSplinePoint _spline_2 _index "Local") (Class|SplineComponent|GetDirectionatSplinePoint _spline_2 _index "Local") (Spline|GetLocationatSplinePoint _spline_2 (+ _index 1) "Local") (Spline|GetArriveTangentatSplinePoint _spline_2 (+ _index 1) "Local") true :!class /Script/Engine.SplineMeshComponent)))

(fn RearrangeCurrentMeshes
  (bind _spline (Variables|Default|GetSpline))
  (bind (_array_element _array_index) (Utilities|Array|ForEachLoopwithBreak (Variables|Default|GetSplineMeshes))
    (:LoopBody
      (Transformation|SetActorLocation (Utilities|Array|Get(acopy) (Variables|Default|GetPhotoParticles) _array_index) (Spline|GetLocationatSplinePoint _spline _array_index "World") false false)
      (SplineMesh|SetStartandEnd _array_element (.Location (Spline|GetLocationandTangentatSplinePoint _spline _array_index "Local")) (.Tangent (Spline|GetLocationandTangentatSplinePoint _spline _array_index "Local")) (.Location (Spline|GetLocationandTangentatSplinePoint _spline (+ _array_index 1) "Local")) (.Tangent (Spline|GetLocationandTangentatSplinePoint _spline (+ _array_index 1) "Local")) true :!class /Script/Engine.SplineMeshComponent))))

(fn RunMapGeneration
  (bind _numremoved (CallFunction|RemoveSplinesfromStart 5))
  (CallFunction|GenerateLevelSpline 1e+03 _numremoved "1.000000, 0,1.000000")
  (CallFunction|RearrangeCurrentMeshes))