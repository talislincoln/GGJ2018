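; Level spawner that places random objects, apparently obstacles, along the BP_LevelManagerV2 spline.
; A half-second looping timer checks each Spawnables entry's time window against elapsed time and spawns a random class from matching entries.
; Actors spawn at the farther spline point of player or last spawn, then jump to a random absolute spline distance.
; They receive CurrentLane, but the lane-offset and rotation helpers are only called from disconnected nodes.
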(event EventBeginPlay
  (bind _outactors (Actor|GetAllActorsOfClass "/Game/Blueprints/BP_Player.BP_Player_C"))
  (if (> (Utilities|Array|Length _outactors) 0)
    (Variables|Default|SetPlayerRef (Utilities|Array|Get(acopy) _outactors))
    (bind _outactors_2 (Actor|GetAllActorsOfClass "/Game/Blueprints/Level/BP_LevelManagerV2.BP_LevelManagerV2_C"))
    (if (> (Utilities|Array|Length _outactors_2) 0)
      (bind _output_get (Variables|Default|SetLevelManagerRef (Utilities|Array|Get(acopy) _outactors_2)))
      (Transformation|SetActorLocation (Transformation|GetActorLocation _output_get) false false)
      (Utilities|Time|SetTimerbyFunctionName self "SpawnObstacles" 0.5 true)
      (Variables|Default|SetLastSpawnedActor (Variables|Default|GetLevelManagerRef)))))

(event Collision|EventActorBeginOverlap
  (params (OtherActor :type Actor%20Object%20Reference)))

(event EventTick
  (params (DeltaSeconds :type Float%20%28single-precision%29))
  (Variables|Default|SetCurrentTimer (+ DeltaSeconds (Variables|Default|GetCurrentTimer))))

(fn ConstructionScript)

(fn SpawnObstacles
  (for _array_element (Variables|Default|GetSpawnables)
    (if (Utilities|InBetween (Variables|Default|GetCurrentTimer) (.StartInterval (Utilities|Struct|BreakS_SpawnStructure _array_element)) (.EndInterval (Utilities|Struct|BreakS_SpawnStructure _array_element)))
      (bind _returnvalue (Game|SpawnActorfromClass (Utilities|Array|Get(acopy) (.ObjectsToSpawn (Utilities|Struct|BreakS_SpawnStructure _array_element)) (Math|Random|RandomIntegerinRange 0 (- (Utilities|Array|Length (.ObjectsToSpawn (Utilities|Struct|BreakS_SpawnStructure _array_element))) 1))) (Math|Transform|MakeTransform (CallFunction|GetSplineLocation) "0, 0, 0" "1,1,1") "Undefined" (Variables|Default|GetLevelManagerRef) 0))
      (Variables|Default|SetLastSpawnedActor _returnvalue)
      (Variables|/Game/Blueprints/Obstacles/BP_BaseObstacle.BP_BaseObstacle_C|SetLane _returnvalue (Variables|Default|GetCurrentLane))
      (Transformation|SetActorTransform _returnvalue (Spline|GetTransformatDistanceAlongSpline (Variables|/Game/Blueprints/Level/BP_LevelManagerV2.BP_LevelManagerV2_C|GetSpline (Variables|Default|GetLevelManagerRef)) (+ (Math|Random|RandomFloatinRange (.StartDistanceInterval (Utilities|Struct|BreakS_SpawnStructure _array_element)) (.EndDistanceInterval (Utilities|Struct|BreakS_SpawnStructure _array_element))) 5e+02) "World" true)))))

(fn GetNextSplineDirection
  (params (Location :type Vector))
  (return (+ (Spline|FindDirectionClosesttoWorldLocation (Variables|/Game/Blueprints/Level/BP_LevelManagerV2.BP_LevelManagerV2_C|GetSpline (Variables|Default|GetLevelManagerRef)) Location "World") (* (* (Class|SplineComponent|FindRightVectorClosesttoWorldLocation (Variables|/Game/Blueprints/Level/BP_LevelManagerV2.BP_LevelManagerV2_C|GetSpline (Variables|Default|GetLevelManagerRef)) Location "World") (Variables|Default|GetCurrentLane)) 1e+02))))

(fn GetSplineLocation
  (if (> (Spline|GetDistanceAlongSplineatSplinePoint (Variables|/Game/Blueprints/Level/BP_LevelManagerV2.BP_LevelManagerV2_C|GetSpline (Variables|Default|GetLevelManagerRef)) (Math|Float|Truncate (Class|SplineComponent|FindInputKeyClosesttoWorldLocation (Variables|/Game/Blueprints/Level/BP_LevelManagerV2.BP_LevelManagerV2_C|GetSpline (Variables|Default|GetLevelManagerRef)) (Transformation|GetActorLocation (Variables|Default|GetPlayerRef))))) (Spline|GetDistanceAlongSplineatSplinePoint (Variables|/Game/Blueprints/Level/BP_LevelManagerV2.BP_LevelManagerV2_C|GetSpline (Variables|Default|GetLevelManagerRef)) (Math|Float|Truncate (Class|SplineComponent|FindInputKeyClosesttoWorldLocation (Variables|/Game/Blueprints/Level/BP_LevelManagerV2.BP_LevelManagerV2_C|GetSpline (Variables|Default|GetLevelManagerRef)) (Transformation|GetActorLocation (Variables|Default|GetLastSpawnedActor))))))
    (return (Spline|FindLocationClosesttoWorldLocation (Variables|/Game/Blueprints/Level/BP_LevelManagerV2.BP_LevelManagerV2_C|GetSpline (Variables|Default|GetLevelManagerRef)) (Transformation|GetActorLocation (Variables|Default|GetPlayerRef)) "World"))
    (else
      (return (Spline|FindLocationClosesttoWorldLocation (Variables|/Game/Blueprints/Level/BP_LevelManagerV2.BP_LevelManagerV2_C|GetSpline (Variables|Default|GetLevelManagerRef)) (Transformation|GetActorLocation (Variables|Default|GetLastSpawnedActor)) "World")))))

(fn GetSplineRotation
  (params (Position :type Vector))
  (return (Class|SplineComponent|FindRotationClosesttoWorldLocation (Variables|/Game/Blueprints/Level/BP_LevelManagerV2.BP_LevelManagerV2_C|GetSpline (Variables|Default|GetLevelManagerRef)) Position "World")))