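; Level manager actor that procedurally generates a winding road along a spline when C is pressed.
; Each press appends points to the spline, stepping by a fixed length in a random direction within a cone around the last tangent.
; It then adds a road spline mesh component per segment, matched to point locations and tangents.
; The SplineMeshes array is cleared but never filled, and earlier mesh components are not destroyed.
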(event EventBeginPlay
  (Input|EnableInput (Game|GetPlayerController 0)))

(event Collision|EventActorBeginOverlap
  (params (OtherActor :type Actor%20Object%20Reference)))

(event EventTick
  (params (DeltaSeconds :type Float%20%28single-precision%29)))

(event Input|KeyboardEvents|C
  (params (Key :type Key%20Structure))
  (:Pressed
    (CallFunction|GenerateLevelSpline 1e+03 100)
    (CallFunction|GenerateLevelSplineMesh)))

(fn ConstructionScript)

(fn GenerateLevelSpline
  (params (RoadLength :type Float%20%28single-precision%29) (NumOfRoad :type Integer))
  (bind _spline (Variables|Default|GetSpline))
  (bind _returnvalue (Spline|GetNumberOfSplinePoints _spline))
  (bind _returnvalue_2 (- _returnvalue 1))
  (for _index (range 0 NumOfRoad)
    (Spline|AddSplinePoint (Variables|Default|GetSpline) (+ (Spline|GetLocationatSplinePoint _spline _returnvalue_2 "Local") (* (Math|Random|RandomUnitVectorinConeinDegrees (Math|Vector|GetForwardVector (Math|Rotator|MakeRotfromX (Spline|GetArriveTangentatSplinePoint _spline _returnvalue_2 "Local"))) 45.0) RoadLength)) "Local" true)))

(fn GenerateLevelSplineMesh
  (bind _spline (Variables|Default|GetSpline))
  (Utilities|Array|Clear (Variables|Default|GetSplineMeshes))
  (for _index (range 0 (- (Spline|GetNumberOfSplinePoints (Variables|Default|GetSpline)) 2))
    (bind _returnvalue (AddComponent|AddSplineMeshComponent false))
    (Components|StaticMesh|SetStaticMesh _returnvalue (Variables|Default|GetRoadMesh))
    (SplineMesh|SetStartandEnd _returnvalue (.Location (Spline|GetLocationandTangentatSplinePoint _spline _index "Local")) (.Tangent (Spline|GetLocationandTangentatSplinePoint _spline _index "Local")) (.Location (Spline|GetLocationandTangentatSplinePoint _spline (+ _index 1) "Local")) (.Tangent (Spline|GetLocationandTangentatSplinePoint _spline (+ _index 1) "Local")) true :!class /Script/Engine.SplineMeshComponent)))