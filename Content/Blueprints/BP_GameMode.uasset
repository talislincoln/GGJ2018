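; Game mode that applies collected powers to players and keeps persistent high score tables for each level.
; Power hit events trigger attached particles, a camera shake and a velocity change; temporary powers are not yet automatically reverted.
; Each level name maps to its own BP_SaveGame slot, loaded or created on BeginPlay and saved on EndPlay.
; AddScore inserts scores by rank and trims each table to ten entries.
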(event Custom|EventApplyPower
  (params (Power :type Base%20Power%20Structure) (PlayerToApply :type BP%20Player%20Object%20Reference))
  (CallFunction|ApplyPowertoPlayer Power PlayerToApply))

(event Custom|AddScore
  (params (NewParam :type BP%20Player%20Object%20Reference) (LevelIndex :type Integer))
  (bind _levelsname (Variables|Default|GetLevelsName))
  (bind _name (Variables|/Game/Blueprints/BP_Player.BP_Player_C|GetName NewParam))
  (bind _levelshighscores (Variables|Default|GetLevelsHighscores))
  (bind _score (Variables|/Game/Blueprints/BP_Player.BP_Player_C|GetScore NewParam))
  (bind _output (Utilities|Array|Get(acopy) _levelsname LevelIndex))
  (bind _scoredata (Utilities|Struct|MakeScoreData _name _score))
  (bind (_value _returnvalue) (Utilities|Map|Find _levelshighscores _output))
  (bind _highscores (Variables|/Game/Blueprints/BP_SaveGame.BP_SaveGame_C|GetHighScores _value))
  (bind _returnvalue_2 (Utilities|Array|Length _highscores))
  (if _returnvalue
    (bind (_array_element _array_index) (Utilities|Array|ForEachLoopwithBreak _highscores :!label _label)
      (:LoopBody
        (if (> (.Score (Utilities|Struct|BreakScoreData _scoredata)) (.Score (Utilities|Struct|BreakScoreData _array_element)))
          (Utilities|Array|Insert _highscores _scoredata _array_index)
          (goto _label Break)))
      (:Completed
        (if (< _array_index (Utilities|Array|Length _highscores))
          (Utilities|Array|Add _highscores _scoredata))
        ;[1 1 1] Remove if more than 10 elements
        (while (> _returnvalue_2 10)
          (Utilities|Array|RemoveIndex _highscores (- _returnvalue_2 1)))))))

(event EventBeginPlay
  (EventDispatchers|BindEventtoOnPowerHit (delegate Custom|EventApplyPower))
  (bind _outactors (Actor|GetAllActorsOfClass "/Game/Blueprints/BP_Player.BP_Player_C"))
  (Variables|Default|SetPlayerRef (Utilities|Array|Get(acopy) _outactors))
  (CallFunction|LoadHighScoresfromFile))

(event EventEndPlay
  (params (EndPlayReason :type EEndPlayReason%20Enum :default "Destroyed"))
  (CallFunction|SaveHighScoresData))

(fn ConstructionScript)

(fn ApplyPowertoPlayer
  (params (Power :type Base%20Power%20Structure) (PlayerToApply :type BP%20Player%20Object%20Reference))
  (Utilities|FlowControl|Sequence
    (:then_1
      ;[1 1 1] Spawn particles
      (Utilities|IsValid (.powerparticles Power)
        (:Is%20Valid
          (Effects|SpawnEmitterAttached (.powerparticles Power) (Variables|/Script/Engine.Actor|GetRootComponent PlayerToApply) "None"))))
    (:then_2
      ;[1 1 1] Play Camera effect
      (if (Utilities|IsValidClass (.cameraeffect Power))
        (Camera|PlayWorldCameraShake (.cameraeffect Power) "0, 0, 0" 0.0 5e+03)))
    (:then_3
      ;[1 0.375 0.375] Update player variables
      (Default|UpdateVelocity PlayerToApply (.velocitymodifier Power))
      (if (.bistemporary Power) ; missing the "remove" power
        _))))

(fn RevertPowerfromPlayer
  (params (Power :type Base%20Power%20Structure) (Player :type BP%20Player%20Object%20Reference))
  (Default|UpdateVelocity Player (/ 1.0 (.velocitymodifier Power))))

(fn SaveHighScoresData
  (for _array_element (Variables|Default|GetLevelsName)
    (SaveGame|SaveGametoSlot (.Value (Utilities|Map|Find (Variables|Default|GetLevelsHighscores) _array_element)) _array_element)))

(fn LoadHighScoresfromFile
  (for _array_element (Variables|Default|GetLevelsName)
    (bind _returnvalue (SaveGame|DoesSaveGameExist _array_element))
    (if _returnvalue
      (bind _returnvalue_2 (SaveGame|LoadGamefromSlot _array_element))
      (bind _asbp_save_game (Utilities|Casting|CastToBP_SaveGame _returnvalue_2))
      (Utilities|Map|Add (Variables|Default|GetLevelsHighscores) _array_element _asbp_save_game)
      (else
        (bind _returnvalue_3 (Game|ConstructObjectfromClass "/Game/Blueprints/BP_SaveGame.BP_SaveGame_C" self))
        (Utilities|Map|Add (Variables|Default|GetLevelsHighscores) _array_element _returnvalue_3)))))

(fn GetHighScores
  (params (LevelIndex :type Integer))
  (return (Variables|/Game/Blueprints/BP_SaveGame.BP_SaveGame_C|GetHighScores (.Value (Utilities|Map|Find (Variables|Default|GetLevelsHighscores) (Utilities|Array|Get(acopy) (Variables|Default|GetLevelsName) LevelIndex))))))